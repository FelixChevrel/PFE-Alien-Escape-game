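; BP_slime_detection is an actor with a box volume that shadows the player's slime character, apparently as its detection area.
; On BeginPlay it caches the player pawn as BP_Slime_Character.
; Each tick it resizes the box from a form-to-extent map keyed by the current form, copies the player's rotation and teleports to the player's location, dropping slightly for one form.
; It contains no active overlap logic.
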(event `self.ReceiveBeginPlay`
  (bind _asbp_slime_character (cast `/Game/Character/Slime/BP_Slime_Character` (`GameplayStatics.GetPlayerPawn` 0)))
  (set `self.player` _asbp_slime_character))

(event `self.ReceiveTick`
  (params (DeltaSeconds :type "Float (single-precision)"))
  (bind _player (`self.player`))
  (`BoxComponent.SetBoxExtent` (`self.Box`) (`BlueprintMapLibrary.Map_Find` (`self.FormByShape`) (`/Game/Character/Slime/BP_Slime_Character.CurrentForm` (`self.player`))) true)
  (`self.K2_SetActorRotation` (`self.K2_GetActorRotation` _player))
  (`self.K2_SetActorLocation` (+ (`self.K2_GetActorLocation` _player) (`KismetMathLibrary.SelectVector` (0.0 0.0 -8.0) (0.0 0.0 0.0) (`|EnumEquality` (`/Game/Character/Slime/BP_Slime_Character.CurrentForm` (`self.player`)) "NewEnumerator3"))) false true))

(fn `UserConstructionScript`)