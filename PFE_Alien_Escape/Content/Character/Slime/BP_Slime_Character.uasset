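; Player slime character that moves relative to the camera, shifts between cube, long and flat forms, and can possess items.
; Held shape inputs play timelines that drive morph targets and slow movement; jumping requires the default form.
; Possessing an overlapped BPI_Possessible attaches it, hides the slime, drops a core and forwards ability input.
; While possessing, long form raises the item, and releasing returns the slime to its core.
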(event `self.ReceiveTick`
  (params (DeltaSeconds :type "Float (single-precision)"))
  (bind _returnvalue (`self.K2_GetActorLocation`))
  (if (or (`self.ForMoving`) (`self.HorMoving`))
    (`SceneComponent.K2_SetWorldRotation` (`self.CapsuleComponent`) (`KismetMathLibrary.FindLookAtRotation` _returnvalue (+ _returnvalue (`KismetMathLibrary.Normal` (`KismetMathLibrary.ProjectVectorOnToPlane` (`MovementComponent.Velocity` (`self.CharacterMovement`)) (0.0 0.0 1.0))))) false false)))

(event `self.ReceiveBeginPlay`
  ;[1 1 1] Set Up
  (set `self.BaseSpeed` (`CharacterMovementComponent.MaxWalkSpeed` (`self.CharacterMovement`))))

(event `InputAxis|Forward`
  (params (AxisValue :type "Float (single-precision)"))
  ;[1 1 1] Base Movement
  (set `self.ForMoving` (!= AxisValue 0.0))
  (`PawnMovementComponent.AddInputVector` (`self.CharacterMovement`) (* (`KismetMathLibrary.Normal` (`KismetMathLibrary.ProjectVectorOnToPlane` (`SceneComponent.GetForwardVector` (`CameraActor.CameraComponent` (`self.Camera`))) (0.0 0.0 1.0))) AxisValue (`self.SpeedMult`) (`KismetMathLibrary.SelectFloat` 0.5 1.0 (`self.InPossession`))) false))

(event `InputAxis|lateral`
  (params (AxisValue :type "Float (single-precision)"))
  ;[1 1 1] Base Movement
  (set `self.HorMoving` (!= AxisValue 0.0))
  (`PawnMovementComponent.AddInputVector` (`self.CharacterMovement`) (* (`KismetMathLibrary.Normal` (`KismetMathLibrary.ProjectVectorOnToPlane` (`SceneComponent.GetRightVector` (`CameraActor.CameraComponent` (`self.Camera`))) (0.0 0.0 1.0))) AxisValue (`self.SpeedMult`) (`KismetMathLibrary.SelectFloat` 0.5 1.0 (`self.InPossession`))) false))

(event `InputAction|ShapeCube`
  (params (Key :type "Key Structure"))
  (bind _mesh (`self.Mesh`))
  (:`Pressed`
    (if (not (`self.InPossession`))
      (set `self.CurrentForm` "NewEnumerator1")
      ;[1 1 1] Shape changing
      (`|ExecutionSequence`
        (:`then_0`
          (bind (_direction _value) (`Timeline|LongTransform` :!via `Reverse` :!label _label)
            (:`Update`
              (if (`self.InPossession`)
                (`SceneComponent.K2_SetRelativeLocation` (`self.ItemAttach`) (`KismetMathLibrary.MakeVector` 0.0 0.0 (+ (* _value 500.0) 150.0)) false false)
                (else
                  (`SkeletalMeshComponent.SetMorphTarget` _mesh "Long" (* _value 1.1) false)
                  (set `self.SpeedMult` (- 1.0 _value)))))))
        (:`then_1`
          (bind (_direction_2 _value_2) (`Timeline|CubeTransform` :!label _label_2)
            (:`Update`
              (`SkeletalMeshComponent.SetMorphTarget` _mesh "MorphTarget_0" _value_2 false)
              (set `self.SpeedMult` (- 1.0 _value_2)))))
        (:`then_2`
          (bind (_direction_3 _value_3) (`Timeline|FlatTransform` :!via `Reverse` :!label _label_3)
            (:`Update`
              (`SkeletalMeshComponent.SetMorphTarget` _mesh "Flat" (* _value_3 0.8) false)
              (set `self.SpeedMult` (- 1.0 _value_3))))))))
  (:`Released`
    (set `self.CurrentForm` "NewEnumerator0")
    (goto _label_2 :!via `Reverse`)))

(event `InputAction|ShapeLong`
  (params (Key :type "Key Structure"))
  (:`Pressed`
    (set `self.CurrentForm` "NewEnumerator2")
    ;[1 1 1] Shape changing
    (`|ExecutionSequence`
      (:`then_0`
        (goto _label_2 :!via `Reverse`))
      (:`then_1`
        (goto _label))
      (:`then_2`
        (goto _label_3 :!via `Reverse`))))
  (:`Released`
    (set `self.CurrentForm` "NewEnumerator0")
    (goto _label :!via `Reverse`)))

(event `InputAction|ShapeFlat`
  (params (Key :type "Key Structure"))
  (:`Pressed`
    (if (not (`self.InPossession`))
      (set `self.CurrentForm` "NewEnumerator3")
      ;[1 1 1] Shape changing
      (`|ExecutionSequence`
        (:`then_0`
          (goto _label :!via `Reverse`))
        (:`then_1`
          (goto _label_3))
        (:`then_2`
          (goto _label_2 :!via `Reverse`)))))
  (:`Released`
    (set `self.CurrentForm` "NewEnumerator0")
    (goto _label_3 :!via `Reverse`)))

(event `InputAction|ItemAbility`
  (params (Key :type "Key Structure"))
  (bind _heldobject (`self.HeldObject`))
  (bind _returnvalue (`KismetSystemLibrary.DoesImplementInterface` _heldobject "/Game/GPE/Possessible/BPI_Possessible.BPI_Possessible_C"))
  (:`Pressed`
    ;[1 1 1] Use Item
    (if _returnvalue
      (message `/Game/GPE/Possessible/BPI_Possessible.Action` _heldobject)))
  (:`Released`
    (if _returnvalue
      (message `/Game/GPE/Possessible/BPI_Possessible.StopAction` _heldobject))))

(event `InputAction|Possess`
  (params (Key :type "Key Structure"))
  (bind _possessiontarget (`self.PossessionTarget`))
  (bind _heldobject (`self.HeldObject`))
  ;[1 1 1] Possess activation/deactivation
  (:`Pressed`
    (if (not (`self.InPossession`))
      (if (`KismetSystemLibrary.IsValid` (`self.PossessionTarget`))
        (set `self.HeldObject` _possessiontarget)
        (`self.SetActorEnableCollision` _possessiontarget false)
        (`self.K2_AttachToComponent` _possessiontarget (`self.ItemAttach`) "None" "SnapToTarget" "SnapToTarget" "KeepWorld" false)
        (set `self.InPossession` true)
        (`SceneComponent.SetVisibility` (`self.Mesh`) false false)
        ;;[1 1 1] Drop a core
        (bind _returnvalue (`|SpawnActorFromClass` "/Game/Character/Slime/BP_Slime_Core.BP_Slime_Core_C" (`self.GetTransform`) "Undefined" "OverrideRootScale" null null))
        (set `self.Core` _returnvalue))
      (else
        (`self.SetActorEnableCollision` _heldobject true)
        (`self.K2_DetachFromActor` _heldobject "KeepWorld" "KeepWorld" "KeepWorld")
        (`self.K2_SetActorLocation` _heldobject (+ (`self.K2_GetActorLocation` _heldobject) (* (`SceneComponent.GetForwardVector` (`self.Arrow1`)) 100.0) (* (+ (`self.CurrentHeight`) 40.0) (`KismetMathLibrary.Vector_Down`))) false true)
        (set `self.PossessionTarget` null)
        (set `self.HeldObject` null)
        (set `self.InPossession` false)
        (`SceneComponent.SetVisibility` (`self.Mesh`) true false)
        ;;[1 1 1] Go back to the core
        (`self.K2_SetActorLocation` (`self.K2_GetActorLocation` (`self.Core`)))
        (`self.K2_DestroyActor` (`self.Core`))
        (set `self.Core` null)))))

(event `InputAction|Jump`
  (params (Key :type "Key Structure"))
  (:`Pressed`
    (if (not (or (`self.InPossession`) (`|EnumInequality` (`self.CurrentForm`) "NewEnumerator0")))
      (`self.Jump`)))
  (:`Released`
    (`self.StopJumping`)))

(event `self.CatchCollision.OnComponentBeginOverlap`
  (params (OverlappedComponent :type "PrimitiveComponent Object Reference") (OtherActor :type "Actor Object Reference") (OtherComp :type "PrimitiveComponent Object Reference") (OtherBodyIndex :type Integer) (bFromSweep :type Boolean) (SweepResult :type "HitResult Structure (by ref)"))
  ;[1 1 1] Possess activation/deactivation
  (if (`KismetSystemLibrary.DoesImplementInterface` OtherActor "/Game/GPE/Possessible/BPI_Possessible.BPI_Possessible_C")
    (set `self.PossessionTarget` OtherActor)))

(fn `AdjustHeight`
  (params (Goal :type "Float (double-precision)"))
  (bind _charactermovement (`self.CharacterMovement`))
  (bind _basespeed (`self.BaseSpeed`))
  (set `self.CurrentHeight` (`KismetMathLibrary.Lerp` (`self.CurrentHeight`) Goal (`self.ShiftingSpeed`)))
  (set `CharacterMovementComponent.MaxWalkSpeed` (`KismetMathLibrary.Lerp` (`MovementComponent.GetMaxSpeed` _charactermovement) (`KismetMathLibrary.SelectFloat` _basespeed (* _basespeed (`self.ShapeSpeedRatio`)) (== Goal 0.0)) (`self.ShiftingSpeed`)) _charactermovement))

(fn `AdjustWidth`
  (params (goal :type "Float (double-precision)"))
  (set `self.CurrentWidth` (`KismetMathLibrary.Lerp` (`self.CurrentWidth`) goal (`self.ShiftingSpeed`))))

(fn `UserConstructionScript`)