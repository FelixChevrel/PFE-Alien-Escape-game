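; Player slime character with camera-relative movement and a squash-and-stretch jump mechanic.
; The Shape axis lerps height, width and walk speed; squashing charges jump power, which stretching releases and neutral resets after a short delay.
; A per-tick forward box trace halts horizontal velocity at obstacles and eases input strength toward zero.
; Surfaces tagged "sticky" also damp vertical velocity and turn the jump into a launch away from the wall.
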(event `self.ReceiveBeginPlay`
  (set `self.BaseSpeed` (`CharacterMovementComponent.MaxWalkSpeed` (`self.CharacterMovement`))))

(event `self.ReceiveTick`
  (params (DeltaSeconds :type "Float (single-precision)"))
  (bind _returnvalue (`self.K2_GetActorLocation`))
  (bind _speedmult (`self.SpeedMult`))
  (`|ExecutionSequence`
    (:`then_0`
      (if (or (`self.ForMoving`) (`self.HorMoving`))
        (`SceneComponent.K2_SetWorldRotation` (`self.CapsuleComponent`) (`KismetMathLibrary.FindLookAtRotation` _returnvalue (+ _returnvalue (`KismetMathLibrary.Normal` (`KismetMathLibrary.ProjectVectorOnToPlane` (`MovementComponent.Velocity` (`self.CharacterMovement`)) (0.0 0.0 1.0))))) false false)))
    (:`then_1`
      (`self.Imobility`
        (:`Move`
          (set `self.SpeedMult` (`KismetMathLibrary.Lerp` _speedmult 1.0 DeltaSeconds)))
        (:`NoMove`
          (set `self.SpeedMult` (`KismetMathLibrary.Lerp` _speedmult 0.0 DeltaSeconds)))))))

(event `InputAxis|Forward`
  (params (AxisValue :type "Float (single-precision)"))
  ;[1 1 1] Base Movement
  (set `self.ForMoving` (!= AxisValue 0.0))
  (`PawnMovementComponent.AddInputVector` (`self.CharacterMovement`) (* (`KismetMathLibrary.Normal` (`KismetMathLibrary.ProjectVectorOnToPlane` (`SceneComponent.GetForwardVector` (`CameraActor.CameraComponent` (`self.Camera`))) (0.0 0.0 1.0))) AxisValue (`self.SpeedMult`)) false))

(event `InputAxis|lateral`
  (params (AxisValue :type "Float (single-precision)"))
  ;[1 1 1] Base Movement
  (set `self.HorMoving` (!= AxisValue 0.0))
  (`PawnMovementComponent.AddInputVector` (`self.CharacterMovement`) (* (`KismetMathLibrary.Normal` (`KismetMathLibrary.ProjectVectorOnToPlane` (`SceneComponent.GetRightVector` (`CameraActor.CameraComponent` (`self.Camera`))) (0.0 0.0 1.0))) AxisValue (`self.SpeedMult`)) false))

(event `InputAxis|Shape`
  (params (AxisValue :type "Float (single-precision)"))
  (bind _returnvalue (`self.K2_GetActorLocation`))
  (bind _launchdirection (`self.LaunchDirection`))
  (bind _jumpready (`self.JumpReady`))
  (bind _nextjumppower (`self.NextJumpPower`))
  ;[1 1 1] Shape Changing mechanic
  (switch `int` (`KismetMathLibrary.Round` AxisValue)
    (:`-1`
      (`self.AdjustHeight` (`self.MinHeight`))
      (`self.AdjustWidth` (`self.MaxWidth`))
      (set `self.JumpReady` true)
      (set `self.NextJumpPower` (`KismetMathLibrary.FClamp` (+ (`self.NextJumpPower`) 25.0) 200.0 (`self.MaxJumpPower`))))
    (:`0`
      (`self.AdjustHeight` 0.0)
      (`self.AdjustWidth` 0.0)
      (`/Engine/EditorBlueprintResources/StandardMacros.DoOnce` false :!label _label
        (:`Completed`
          (`KismetSystemLibrary.Delay` 0.25)
          (set `self.JumpReady` false)
          (set `self.NextJumpPower` 200.0)
          (goto _label :!via `Reset`))))
    (:`1`
      (`self.AdjustHeight` (`self.MaxHeight`))
      (`self.AdjustWidth` (`self.MinWidth`))
      (if (not (`self.OnWall`))
        (if _jumpready
          (set `CharacterMovementComponent.JumpZVelocity` _nextjumppower (`self.CharacterMovement`))
          (set `self.NextJumpPower` 200.0)
          (`self.Jump`)
          (set `self.JumpReady` false))
        (elif _jumpready
          (`self.LaunchCharacter` (* _launchdirection (* _nextjumppower 1.25)) true true)
          (`SceneComponent.K2_SetWorldRotation` (`self.CapsuleComponent`) (`KismetMathLibrary.FindLookAtRotation` _returnvalue (+ _returnvalue (`KismetMathLibrary.ProjectVectorOnToPlane` _launchdirection (0.0 0.0 1.0)))) false false))))))

(fn `AdjustHeight`
  (params (Goal :type "Float (double-precision)"))
  (bind _charactermovement (`self.CharacterMovement`))
  (bind _basespeed (`self.BaseSpeed`))
  (set `self.CurrentHeight` (`KismetMathLibrary.Lerp` (`self.CurrentHeight`) Goal (`self.ShiftingSpeed`)))
  (set `CharacterMovementComponent.MaxWalkSpeed` (`KismetMathLibrary.Lerp` (`MovementComponent.GetMaxSpeed` _charactermovement) (`KismetMathLibrary.SelectFloat` _basespeed (* _basespeed (`self.ShapeSpeedRatio`)) (== Goal 0.0)) (`self.ShiftingSpeed`)) _charactermovement))

(fn `AdjustWidth`
  (params (goal :type "Float (double-precision)"))
  (set `self.CurrentWidth` (`KismetMathLibrary.Lerp` (`self.CurrentWidth`) goal (`self.ShiftingSpeed`))))

(fn `UserConstructionScript`)