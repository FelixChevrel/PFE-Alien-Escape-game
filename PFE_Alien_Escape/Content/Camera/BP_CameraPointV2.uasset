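; Rail-style camera that moves a CAMERA actor along authored points as the BP_Slime_Character advances along a parallel player path.
; Each Tick, CheckPlayerPosition projects the player onto the current PlayerPoint segment for a signed blend, stepping CurrentID when it leaves the segment.
; The camera eases toward that blend between matching CameraPoints.
; A Copy toggle seeds CameraPoints above PlayerPoints; BeginPlay draws debug boxes and loops an empty CheckPositions timer.
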(event `self.ReceiveBeginPlay`
  (`|ExecutionSequence`
    (:`then_0`
      (bind _asbp_slime_character (cast `/Game/Character/Slime/BP_Slime_Character` (`GameplayStatics.GetPlayerPawn` 0)))
      (set `self.player` _asbp_slime_character)
      (for _array_element (`self.PlayerPoint`)
        (`KismetSystemLibrary.DrawDebugBox` (+ _array_element (`self.K2_GetActorLocation`)) (100.0 100.0 100.0) (struct :`R` 1.0 :`A` 1.0) (struct) 100.0 10.0)))
    (:`then_1`
      (`KismetSystemLibrary.K2_SetTimerDelegate` (delegate `CheckPositions`) 0.1 true))))

(event `CheckPositions`)

(event `self.ReceiveTick`
  (params (DeltaSeconds :type "Float (single-precision)"))
  (bind _returnvalue (`self.K2_GetActorLocation`))
  (bind _currentid (`self.CurrentID`))
  (bind _camerapoint (`self.CameraPoint`))
  (bind _camera (`self.CAMERA`))
  (`|ExecutionSequence`
    (:`then_0`
      (`self.CheckPlayerPosition`))
    (:`then_1`
      ;[1 1 1] Set camera location
      (`self.K2_SetActorLocation` _camera (`KismetMathLibrary.VLerp` (`self.K2_GetActorLocation` _camera) (`KismetMathLibrary.VLerp` (+ (`|GetArrayItem` _camerapoint _currentid) _returnvalue) (+ _returnvalue (`|GetArrayItem` _camerapoint (+ _currentid 1))) (`self.CurrentBlendValue`)) DeltaSeconds) false false))))

(fn `UserConstructionScript`
  (if (`self.Copy`)
    (`KismetArrayLibrary.Array_Clear` (`self.CameraPoint`))
    (set `self.Copy` false)
    (for _array_element (`self.PlayerPoint`)
      (`KismetArrayLibrary.Array_Add` (`self.CameraPoint`) (+ _array_element (0.0 0.0 500.0))))))