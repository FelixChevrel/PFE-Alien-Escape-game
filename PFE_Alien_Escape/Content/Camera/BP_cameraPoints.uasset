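; BP_cameraPoints is a camera point that repositions the game camera when the player enters its detection volume.
; BeginPlay caches the player 0 pawn, and the PlayerDetection overlap responds only to that actor.
; On overlap it passes the world transform of its Attach component to the referenced Camera, calls that camera's Attach, then sets its goal field of view from the point's FOVPoint.
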(event `self.ReceiveBeginPlay`
  (set `self.Player` (`GameplayStatics.GetPlayerPawn` 0)))

(event `self.PlayerDetection.OnComponentBeginOverlap`
  (params (OverlappedComponent :type "PrimitiveComponent Object Reference") (OtherActor :type "Actor Object Reference") (OtherComp :type "PrimitiveComponent Object Reference") (OtherBodyIndex :type Integer) (bFromSweep :type Boolean) (SweepResult :type "HitResult Structure (by ref)"))
  (bind _camera (`self.Camera`))
  (if (== OtherActor (`self.Player`))
    (set `/Game/Camera/BPC_Camera.CurrentAttach` (`SceneComponent.K2_GetComponentToWorld` (`self.Attach`)) _camera)
    (`/Game/Camera/BPC_Camera.Attach` _camera)
    (set `/Game/Camera/BPC_Camera.GoalFoV` (`self.FOVPoint`) _camera)))

(fn `UserConstructionScript`)