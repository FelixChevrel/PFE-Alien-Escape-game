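; Camera actor that tracks the player and glides between attach points.
; Attach detaches the actor, then a Move timeline blends its transform toward CurrentAttach and field of view toward GoalFoV.
; Each tick, the scene component turns toward the player at a rate shaped by a curve over view alignment.
; The camera component separately eases pitch and yaw offsets driven by BlendY and BlendX.
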(event `Attach`
  (bind _cameracomponent (`self.CameraComponent`))
  ;[1 1 1] Attach to point
  (`self.K2_DetachFromActor` "KeepWorld" "KeepWorld" "KeepWorld")
  (`TimelineComponent.SetPlayRate` (`self.Move`) 1.0)
  (bind (_direction _smooth_adjustement _arm_length) (`Timeline|Move` :!via `PlayFromStart`)
    (:`Update`
      (`self.K2_SetActorTransform` (`KismetMathLibrary.TLerp` (`self.GetTransform`) (`self.CurrentAttach`) _smooth_adjustement))
      (`CameraComponent.SetFieldOfView` _cameracomponent (`KismetMathLibrary.Lerp` (`CameraComponent.FieldOfView` _cameracomponent) (`self.GoalFoV`) _arm_length)))
    (:`Finished`
      (`KismetSystemLibrary.PrintString` "End"))))

(event `self.ReceiveTick`
  (params (DeltaSeconds :type "Float (single-precision)"))
  (bind _scenecomponent (`self.SceneComponent`))
  (bind _cameracomponent (`self.CameraComponent`))
  (bind _returnvalue (`SceneComponent.K2_GetComponentRotation` _scenecomponent))
  (bind (_relativerotation_roll _relativerotation_pitch _relativerotation_yaw) (`KismetMathLibrary.BreakRotator` (`SceneComponent.RelativeRotation` _cameracomponent)))
  (bind _returnvalue_2 (`KismetMathLibrary.FindLookAtRotation` (`SceneComponent.K2_GetComponentLocation` (`self.SceneComponent`)) (`self.K2_GetActorLocation` (`self.Player`))))
  (`SceneComponent.K2_SetWorldRotation` _scenecomponent (`KismetMathLibrary.RLerp` _returnvalue _returnvalue_2 (* (`CurveFloat.GetFloatValue` (`self.CurveSlow`) (`KismetMathLibrary.Dot_VectorVector` (`KismetMathLibrary.GetForwardVector` _returnvalue_2) (`KismetMathLibrary.GetForwardVector` _returnvalue))) DeltaSeconds 2.0) true) false false)
  (`SceneComponent.K2_SetRelativeRotation` _cameracomponent (`KismetMathLibrary.MakeRotator` 0.0 (`KismetMathLibrary.Lerp` _relativerotation_pitch (`KismetMathLibrary.Lerp` 0.0 20.0 (`self.BlendY`)) DeltaSeconds) (`KismetMathLibrary.Lerp` _relativerotation_yaw (`KismetMathLibrary.Lerp` 0.0 20.0 (`self.BlendX`)) DeltaSeconds)) false false))

(fn `UserConstructionScript`)