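; BP_Hunter_detection_Lazer is a Hunter laser detector that signals when an actor tagged Player is in its line of fire.
; A looping one-second timer runs a sphere trace on the Visibility channel forward along the Arrow component.
; The Sphere mesh turns glowing green when the hit actor carries the Player tag, and black otherwise.
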(event `self.ReceiveBeginPlay`
  (`KismetSystemLibrary.K2_SetTimerDelegate` (delegate `Check`) 1.0 true))

(event `Check`
  (bind _returnvalue (`self.K2_GetActorLocation`))
  (bind _sphere (`self.Sphere`))
  (bind _returnvalue_2 (`SceneComponent.GetForwardVector` (`self.arrow`)))
  (bind (_outhit _returnvalue_3) (`KismetSystemLibrary.SphereTraceSingle` :`Start` (+ _returnvalue (* _returnvalue_2 100.0)) :`End` (+ _returnvalue (* _returnvalue_2 1000.0)) :`Radius` 15.0 :`TraceChannel` "TraceTypeQuery1" :`DrawTime` 1.0))
  (if _returnvalue_3
    (if (`self.ActorHasTag` (`.HitActor` (`GameplayStatics.BreakHitResult` _outhit)) "Player")
      (`PrimitiveComponent.SetMaterial` _sphere 0 "/Game/Material/MATINST_glow_green.MATINST_glow_green")
      (else
        (`PrimitiveComponent.SetMaterial` _sphere 0 "/Game/Material/Drill/MAT_black.MAT_black" :!label _label)))
    (else
      (goto _label))))

(fn `UserConstructionScript`)