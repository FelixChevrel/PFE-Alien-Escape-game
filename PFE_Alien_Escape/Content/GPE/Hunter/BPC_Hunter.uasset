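; Hunter enemy character that ends the game by pausing it when its hit collision touches the player or slime core.
; Tick mirrors the AI controller's color state onto its spotlight and indicator material, and resets walk speed to regular.
; Overlapping a Destructible actor once triggers a brief slowdown and spawns a scaled-up destruction actor at the hunter.
; A SingularScan macro, unused here, sphere-traces forward to catch the player.
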(event `self.ReceiveTick`
  (params (DeltaSeconds :type "Float (single-precision)"))
  (bind _asaic_hunter (cast `/Game/GPE/Hunter/AIC_Hunter` (`self.GetController`))
    (:`then`
      (bind _color (`/Game/GPE/Hunter/AIC_Hunter.Color` _asaic_hunter))
      (`LightComponent.SetLightColor` (`self.SpotLight`) (select `int` _color :`0` (struct :`R` 1.0 :`G` 1.0 :`B` 1.0 :`A` 1.0) :`1` (struct :`R` 0.823201 :`G` 1.0 :`A` 1.0) :`2` (struct :`R` 1.0 :`G` 0.076232 :`A` 1.0) :!type "LinearColor Structure") true)
      (`PrimitiveComponent.SetMaterial` (`self.LightIndicator`) 0 (select `int` _color :`0` "/Game/Material/MATINST_glow_green.MATINST_glow_green" :`1` "/Game/Material/MATINST_glow_yellow.MATINST_glow_yellow" :`2` "/Game/Material/MAT_glow.MAT_glow" :!type "MaterialInterface Object Reference"))
      (set `CharacterMovementComponent.MaxWalkSpeed` (`self.RegularSpeed`) (`self.CharacterMovement`)))
    (:`CastFailed`
      (`KismetSystemLibrary.PrintString` "Error"))))

(event `self.HitCollision.OnComponentBeginOverlap`
  (params (OverlappedComponent :type "PrimitiveComponent Object Reference") (OtherActor :type "Actor Object Reference") (OtherComp :type "PrimitiveComponent Object Reference") (OtherBodyIndex :type Integer) (bFromSweep :type Boolean) (SweepResult :type "HitResult Structure (by ref)"))
  (bind (_returnvalue_location _returnvalue_rotation _returnvalue_scale) (`KismetMathLibrary.BreakTransform` (`self.GetTransform`)))
  (if (or (== OtherActor (`GameplayStatics.GetPlayerPawn` 0)) (== (`GameplayStatics.GetObjectClass` OtherActor) "/Game/Character/Slime/BP_Slime_Core.BP_Slime_Core_C"))
    (`KismetSystemLibrary.PrintString` "Game Over")
    (`GameplayStatics.SetGamePaused` true)
    (elif (`self.ActorHasTag` OtherActor "Destructible")
      (`/Engine/EditorBlueprintResources/StandardMacros.DoOnce` false
        (:`Completed`
          (set `CharacterMovementComponent.MaxWalkSpeed` (`self.SlowSpeed`) (`self.CharacterMovement`))
          (`KismetSystemLibrary.Delay` 0.2)
          (`|SpawnActorFromClass` "/Game/GPE/Fields/FS_Robot_Destruction.FS_Robot_Destruction_C" (`KismetMathLibrary.MakeTransform` _returnvalue_location _returnvalue_rotation (* _returnvalue_scale (2.0 2.0 2.0))) "Undefined" "OverrideRootScale" null null)
          (`KismetSystemLibrary.Delay` 0.8)
          (set `CharacterMovementComponent.MaxWalkSpeed` (`self.RegularSpeed`) (`self.CharacterMovement`)))))))

(fn `UserConstructionScript`)