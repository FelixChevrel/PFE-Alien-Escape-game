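; Hiding spot that snaps the slime player into place when it enters the spot in the matching form.
; A looping timer polls for overlap and checks the player's CurrentForm against GoodShape.
; On a match, a one-shot timeline lerps the player to the Arrow's horizontal position and rotation and applies the hidden slime material.
; A wrong form stops the timeline; either that or leaving re-arms the one-shot.
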(event `self.ReceiveBeginPlay`
  (bind _asbp_slime_character (cast `/Game/Character/Slime/BP_Slime_Character` (`GameplayStatics.GetPlayerPawn` 0)))
  (set `self.Player` _asbp_slime_character)
  (`KismetSystemLibrary.K2_SetTimerDelegate` (delegate `Adjust`) 0.1 true))

(event `Adjust`
  (bind _player (`self.Player`))
  (bind _arrow (`self.Arrow`))
  (bind _player_2 (`self.Player`))
  (bind (_returnvalue_x _returnvalue_y) (`KismetMathLibrary.BreakVector` (`SceneComponent.K2_GetComponentLocation` _arrow)))
  (bind (_returnvalue_location _returnvalue_rotation _returnvalue_scale) (`KismetMathLibrary.BreakTransform` (`self.GetTransform` _player_2)))
  (if (`PrimitiveComponent.IsOverlappingActor` (`self.Root`) _player)
    (if (`|EnumEquality` (`/Game/Character/Slime/BP_Slime_Character.CurrentForm` _player) (`self.GoodShape`))
      (`/Engine/EditorBlueprintResources/StandardMacros.DoOnce` false :!label _label
        (:`Completed`
          (bind (_direction _lerp) (`Timeline|MoveToSpot` :!via `PlayFromStart` :!label _label_2)
            (:`Update`
              (`self.K2_SetActorTransform` _player_2 (`KismetMathLibrary.MakeTransform` (`KismetMathLibrary.VLerp` _returnvalue_location (`KismetMathLibrary.MakeVector` _returnvalue_x _returnvalue_y (.z _returnvalue_location)) _lerp) (`KismetMathLibrary.RLerp` _returnvalue_rotation (`SceneComponent.K2_GetComponentRotation` _arrow) _lerp true) _returnvalue_scale) false false)
              (`PrimitiveComponent.SetMaterial` (`Character.Mesh` (`self.Player`)) 0 "/Game/Material/MATINST_Slime_hidden.MATINST_Slime_hidden")))))
      (else
        (`|ExecutionSequence`
          (:`then_0`
            (goto _label_2 :!via `Stop`))
          (:`then_1`
            (goto _label :!via `Reset`)))))
    (else
      (goto _label :!via `Reset`))))

(fn `UserConstructionScript`)