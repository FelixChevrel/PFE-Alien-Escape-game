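; BP_Saw is a possessable saw that the slime player can take over and use to cut procedural meshes.
; Attach leaves a BP_Slime_Core at the player's spot, moves the player to the saw and mounts it on ItemAttach.
; Detach drops the saw, returns the player to the core and destroys it.
; Action line-traces forward, slices the hit ProceduralMeshComponent with a wood cap and launches the new half sideways as a physics body.
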(event `self.ReceiveBeginPlay`
  (bind _asbp_slime_character (cast `/Game/Character/Slime/BP_Slime_Character` (`GameplayStatics.GetPlayerPawn` 0)))
  (set `self.Player` _asbp_slime_character))

(event `/Game/GPE/Possessible/BPI_Possessible.Attach`
  (bind (_returnvalue_location _returnvalue_rotation) (`KismetMathLibrary.BreakTransform` (`self.GetTransform`)))
  (bind _player (`self.Player`))
  (bind _player_2 (`self.Player`))
  (if (not (`self.Equiped`))
    (set `self.Equiped` true)
    (bind _returnvalue (`|SpawnActorFromClass` "/Game/Character/Slime/BP_Slime_Core.BP_Slime_Core_C" (`self.GetTransform` _player) "Undefined" "OverrideRootScale" null null))
    (set `/Game/Character/Slime/BP_Slime_Character.Core` _returnvalue _player)
    (set `/Game/Character/Slime/BP_Slime_Character.HeldObject` self _player)
    (`self.K2_SetActorTransform` _player_2 (`KismetMathLibrary.MakeTransform` _returnvalue_location _returnvalue_rotation) false false)
    (set `/Game/Character/Slime/BP_Slime_Character.InPossession` true _player_2)
    (`self.K2_AttachToComponent` (`/Game/Character/Slime/BP_Slime_Character.ItemAttach` _player_2) "None" "SnapToTarget" "SnapToTarget" "KeepWorld" false)
    (`SceneComponent.K2_AddRelativeRotation` (`self.Cube1`) (struct :`Yaw` 90.0) false false)))

(event `/Game/GPE/Possessible/BPI_Possessible.Detach`
  (bind _player (`self.Player`))
  (bind _core (`/Game/Character/Slime/BP_Slime_Character.Core` _player))
  (if (`self.Equiped`)
    (`self.K2_DetachFromActor` "KeepWorld" "KeepWorld" "KeepWorld")
    (`self.K2_SetActorLocation` (- (`self.K2_GetActorLocation`) (0.0 0.0 50.0)))
    (set `self.Equiped` false)
    (`self.K2_SetActorLocation` _player (`self.K2_GetActorLocation` _core) false false)
    (`self.K2_DestroyActor` _core)
    (set `/Game/Character/Slime/BP_Slime_Character.InPossession` false _player)
    (set `/Game/Character/Slime/BP_Slime_Character.HeldObject` null _player)
    (set `/Game/Character/Slime/BP_Slime_Character.Core` null _player)))

(event `/Game/GPE/Possessible/BPI_Possessible.Action`
  (bind _returnvalue (`SceneComponent.K2_GetComponentLocation` (`self.Arrow`)))
  (bind _returnvalue_2 (`SceneComponent.GetForwardVector` (`self.Arrow`)))
  (bind (_outhit _returnvalue_3) (`KismetSystemLibrary.LineTraceSingle` _returnvalue (+ _returnvalue (* (`self.GetActorForwardVector`) 250.0)) "TraceTypeQuery1" false (`|MakeArray` (`self.Player`) :!type "Actor Object Reference") "ForDuration"))
  (if _returnvalue_3
    (bind (_bblockinghit _binitialoverlap _time _distance _location _impactpoint _normal _impactnormal _physmat _hitactor _hitcomponent) (`GameplayStatics.BreakHitResult` _outhit))
    (bind _asprocedural_mesh_component (cast `ProceduralMeshComponent` _hitcomponent))
    (`PrimitiveComponent.SetSimulatePhysics` _asprocedural_mesh_component true)
    (bind _outotherhalfprocmesh (`KismetProceduralMeshLibrary.SliceProceduralMesh` _asprocedural_mesh_component _impactpoint _returnvalue_2 true "CreateNewSectionForCap" "/Game/Material/MATINST_Wood.MATINST_Wood"))
    (`PrimitiveComponent.SetCollisionEnabled` _outotherhalfprocmesh "QueryAndPhysics")
    (`PrimitiveComponent.SetMassScale` _outotherhalfprocmesh "None" 0.1)
    (`PrimitiveComponent.SetCollisionObjectType` _outotherhalfprocmesh "ECC_GameTraceChannel1")
    (`PrimitiveComponent.SetSimulatePhysics` _outotherhalfprocmesh true)
    (`PrimitiveComponent.AddImpulse` _outotherhalfprocmesh (* (`KismetMathLibrary.RotateAngleAxis` _returnvalue_2 90.0 (0.0 0.0 1.0)) 500.0) "None" true)))

(event `/Game/GPE/Possessible/BPI_Possessible.StopAction`)

(fn `UserConstructionScript`)