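; BP_Crane is a crane the slime player can possess to pick up and drop objects.
; Attach spawns a slime core at the player's transform, moves the player to the crane and attaches to it; Detach returns the player to the core and destroys it.
; Action lowers and raises the grip, releasing any held object.
; Grip zone overlaps attach "Grabbable"-tagged actors to the grip point and disable the zone's collision until the next Action.
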(event `self.ReceiveBeginPlay`
  (bind _asbp_slime_character (cast `/Game/Character/Slime/BP_Slime_Character` (`GameplayStatics.GetPlayerPawn` 0)))
  (set `self.PlayerRef` _asbp_slime_character))

(event `/Game/GPE/Possessible/BPI_Possessible.Attach`
  (bind _returnvalue (`self.GetTransform`))
  (bind _playerref (`self.PlayerRef`))
  (bind _playerref_2 (`self.PlayerRef`))
  (if (not (`self.Equiped`))
    (set `self.Equiped` true)
    (bind _returnvalue_2 (`|SpawnActorFromClass` "/Game/Character/Slime/BP_Slime_Core.BP_Slime_Core_C" (`self.GetTransform` _playerref) "Undefined" "OverrideRootScale" null null))
    (set `/Game/Character/Slime/BP_Slime_Character.Core` _returnvalue_2 _playerref)
    (set `/Game/Character/Slime/BP_Slime_Character.HeldObject` self _playerref)
    (`self.K2_SetActorTransform` _playerref_2 (`KismetMathLibrary.MakeTransform` (`KismetMathLibrary.MakeVector` (.x (.location _returnvalue)) (.y (.location _returnvalue)) (- (.z (.location _returnvalue)) 20.0)) (.rotation _returnvalue)) false false)
    (set `/Game/Character/Slime/BP_Slime_Character.InPossession` true _playerref_2)
    (`self.K2_AttachToComponent` (`/Game/Character/Slime/BP_Slime_Character.ItemAttach` _playerref_2) "None" "SnapToTarget" "SnapToTarget" "KeepWorld" false)))

(event `/Game/GPE/Possessible/BPI_Possessible.Detach`
  (bind _playerref (`self.PlayerRef`))
  (bind _core (`/Game/Character/Slime/BP_Slime_Character.Core` _playerref))
  (if (`self.Equiped`)
    (`self.K2_DetachFromActor` "KeepWorld" "KeepWorld" "KeepWorld")
    (`self.K2_SetActorLocation` (- (`self.K2_GetActorLocation`) (0.0 0.0 50.0)))
    (set `self.Equiped` false)
    (`self.K2_SetActorLocation` _playerref (`self.K2_GetActorLocation` _core) false false)
    (`self.K2_DestroyActor` _core)
    (set `/Game/Character/Slime/BP_Slime_Character.InPossession` false _playerref)
    (set `/Game/Character/Slime/BP_Slime_Character.HeldObject` null _playerref)
    (set `/Game/Character/Slime/BP_Slime_Character.Core` null _playerref)))

(event `/Game/GPE/Possessible/BPI_Possessible.Action`
  (if (`self.IsObjectGrabbed?`)
    (`KismetSystemLibrary.MoveComponentTo` (`self.Grip`) (0.0 0.0 -650.0) (struct :`Yaw` 180.0) false false 1.25)
    (`self.K2_DetachFromActor` (`self.GrabbedObject`) "KeepWorld" "KeepWorld" "KeepWorld")
    (`KismetSystemLibrary.Delay` 0.25)
    (`KismetSystemLibrary.MoveComponentTo` (`self.Grip`) (0.0 0.0 0.0) (struct :`Yaw` 180.0) false false 1.25)
    (`PrimitiveComponent.SetCollisionEnabled` (`self.GripZone`) "QueryAndPhysics")
    (set `self.IsObjectGrabbed?` false)
    (else
      (`KismetSystemLibrary.MoveComponentTo` (`self.Grip`) (0.0 0.0 -650.0) (struct :`Yaw` 180.0) false false 1.25)
      (`KismetSystemLibrary.Delay` 0.25)
      (`KismetSystemLibrary.MoveComponentTo` (`self.Grip`) (0.0 0.0 0.0) (struct :`Yaw` 180.0) false false 1.25)
      (`PrimitiveComponent.SetCollisionEnabled` (`self.GripZone`) "QueryAndPhysics"))))

(event `self.GripZone.OnComponentBeginOverlap`
  (params (OverlappedComponent :type "PrimitiveComponent Object Reference") (OtherActor :type "Actor Object Reference") (OtherComp :type "PrimitiveComponent Object Reference") (OtherBodyIndex :type Integer) (bFromSweep :type Boolean) (SweepResult :type "HitResult Structure (by ref)"))
  (if (`self.IsObjectGrabbed?`)
    _
    (elif (`self.ActorHasTag` OtherActor "Grabbable")
      (set `self.GrabbedObject` OtherActor)
      (set `self.IsObjectGrabbed?` true)
      (`self.K2_AttachToComponent` OtherActor (`self.GripPoint`) "None" "SnapToTarget" "SnapToTarget" "KeepWorld" false)
      (`PrimitiveComponent.SetCollisionEnabled` (`self.GripZone`) "NoCollision"))))

(fn `UserConstructionScript`)