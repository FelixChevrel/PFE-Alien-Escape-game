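; Possessible boat that the slime player takes over to winch up objects from below.
; Attach leaves a BP_Slime_Core behind, mounts the boat on the player and swaps water and hull collision; Detach returns the player to the core.
; A looping timer sphere-traces below the wire and lights the alarm over a target.
; Action alternates between lifting it via the PullUP timeline, which drives player anchoring, and releasing it with physics restored.
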(event `CheckBellow`
  (bind _alarm (`self.Alarm`))
  (bind _returnvalue (`SceneComponent.K2_GetComponentLocation` (`self.Wire`)))
  (if (and (`self.Equiped`) (not (`self.InMotion`)))
    (bind (_outhit _returnvalue_2) (`KismetSystemLibrary.SphereTraceSingle` _returnvalue (+ _returnvalue (0.0 0.0 -1500.0)) 85.0 "TraceTypeQuery3" false (`|MakeArray` (`self.Player`) :!type "Actor Object Reference")))
    (if _returnvalue_2
      (set `self.StuffToPullUp` (`.HitActor` (`GameplayStatics.BreakHitResult` _outhit)))
      (`PrimitiveComponent.SetMaterial` _alarm 0 "/Game/Material/Drill/MAT_Battery.MAT_Battery")
      (else
        (set `self.StuffToPullUp` null)
        (`PrimitiveComponent.SetMaterial` _alarm 0 "/Game/Material/Drill/MAT_black.MAT_black")))))

(event `/Game/GPE/Possessible/BPI_Possessible.Action`
  (bind _stufftopullup (`self.StuffToPullUp`))
  (bind _stufftopullup_2 (`self.StuffToPullUp`))
  (bind _player (`self.Player`))
  (if (`KismetSystemLibrary.IsValid` (`self.StuffToPullUp`))
    (`/Engine/EditorBlueprintResources/StandardMacros.FlipFlop`
      (:`A`
        (set `/Game/Character/Slime/BP_Slime_Character.Anchored` false _player)
        (`self.SetActorEnableCollision` _stufftopullup_2 false)
        (message `/Game/GPE/Water/BPI_Floater.ActivatePhysic` _stufftopullup_2 false)
        (set `self.InMotion` true)
        (bind (_direction _newtrack_0 _newtrack_2) (`Timeline|PullUP` :!via `PlayFromStart` :!label _label)
          (:`Update`
            (set `/Game/Character/Slime/BP_Slime_Character.Anchored` (>= _newtrack_2 1.0) (`self.Player`))
            (`self.K2_SetActorLocation` _stufftopullup (`KismetMathLibrary.VLerp` (`self.K2_GetActorLocation` _stufftopullup) (`SceneComponent.K2_GetComponentLocation` (`self.PullPoint`)) _newtrack_0) false false))))
      (:`B`
        (set `/Game/Character/Slime/BP_Slime_Character.Anchored` true _player)
        (`self.SetActorEnableCollision` _stufftopullup_2 true)
        (message `/Game/GPE/Water/BPI_Floater.ActivatePhysic` _stufftopullup_2 true)
        (set `self.InMotion` false)
        (goto _label :!via `Stop`)))))

(event `self.ReceiveBeginPlay`
  (bind _asbp_slime_character (cast `/Game/Character/Slime/BP_Slime_Character` (`GameplayStatics.GetPlayerPawn` 0)))
  (set `self.Player` _asbp_slime_character)
  (`KismetSystemLibrary.K2_SetTimerDelegate` (delegate `CheckBellow`) 0.2 true))

(event `/Game/GPE/Possessible/BPI_Possessible.StopAction`)

(event `/Game/GPE/Possessible/BPI_Possessible.Attach`
  (bind (_returnvalue_location _returnvalue_rotation) (`KismetMathLibrary.BreakTransform` (`self.GetTransform`)))
  (bind _player (`self.Player`))
  (bind _cube (`self.Cube`))
  (bind _player_2 (`self.Player`))
  (bind _cube_2 (`self.Cube`))
  (if (not (`self.Equiped`))
    (set `self.Equiped` true)
    (bind _returnvalue (`|SpawnActorFromClass` "/Game/Character/Slime/BP_Slime_Core.BP_Slime_Core_C" (`self.GetTransform` _player) "Undefined" "OverrideRootScale" null null))
    (set `/Game/Character/Slime/BP_Slime_Character.Core` _returnvalue _player)
    (set `/Game/Character/Slime/BP_Slime_Character.HeldObject` self _player)
    (`KismetSystemLibrary.PrintString` "Hello")
    (`self.K2_SetActorTransform` _player_2 (`KismetMathLibrary.MakeTransform` _returnvalue_location _returnvalue_rotation) false false)
    (set `/Game/Character/Slime/BP_Slime_Character.InPossession` true _player_2)
    (`self.K2_AttachToComponent` (`/Game/Character/Slime/BP_Slime_Character.ItemAttach` _player_2) "None" "SnapToTarget" "SnapToTarget" "KeepWorld" false)
    (`SceneComponent.K2_SetRelativeLocation` _cube_2 (0.0 0.0 -500.0) false false)
    (`SceneComponent.K2_SetRelativeRotation` _cube_2 (struct :`Yaw` 90.0) false false)
    (`PrimitiveComponent.SetCollisionResponseToChannel` (`StaticMeshActor.StaticMeshComponent` (`self.Water-area`)) "ECC_WorldDynamic" "ECR_Block")
    (`PrimitiveComponent.SetCollisionResponseToChannel` _cube "ECC_WorldDynamic" "ECR_Ignore")
    (`PrimitiveComponent.SetCollisionResponseToChannel` _cube "ECC_Pawn" "ECR_Ignore")))

(event `/Game/GPE/Possessible/BPI_Possessible.Detach`
  (bind _cube (`self.Cube`))
  (bind _player (`self.Player`))
  (bind _core (`/Game/Character/Slime/BP_Slime_Character.Core` _player))
  (if (`self.Equiped`)
    (`self.K2_DetachFromActor` "KeepWorld" "KeepWorld" "KeepWorld")
    (`self.K2_SetActorLocation` (- (`self.K2_GetActorLocation`) (0.0 0.0 0.0)))
    (set `self.Equiped` false)
    (`self.K2_SetActorLocation` _player (`self.K2_GetActorLocation` _core) false false)
    (`self.K2_DestroyActor` _core)
    (set `/Game/Character/Slime/BP_Slime_Character.InPossession` false _player)
    (set `/Game/Character/Slime/BP_Slime_Character.HeldObject` null _player)
    (set `/Game/Character/Slime/BP_Slime_Character.Core` null _player)
    (`PrimitiveComponent.SetCollisionResponseToChannel` (`StaticMeshActor.StaticMeshComponent` (`self.Water-area`)) "ECC_WorldDynamic" "ECR_Ignore")
    (`PrimitiveComponent.SetCollisionResponseToChannel` _cube "ECC_WorldDynamic" "ECR_Block")
    (`PrimitiveComponent.SetCollisionResponseToChannel` _cube "ECC_Pawn" "ECR_Block")))

(fn `UserConstructionScript`)