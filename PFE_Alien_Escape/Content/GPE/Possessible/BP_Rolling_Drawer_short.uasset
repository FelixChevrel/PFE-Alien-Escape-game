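; Possessible short rolling drawer that the slime player character can take over and leave.
; Attach spawns a slime core where the player stood, moves the player to the drawer, snaps the drawer to the player's ItemAttach and flags possession.
; Detach drops the drawer slightly lower, returns the player to the core's location, then destroys the core and clears possession state.
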(event `self.ReceiveBeginPlay`
  (bind _asbp_slime_character (cast `/Game/Character/Slime/BP_Slime_Character` (`GameplayStatics.GetPlayerPawn` 0)))
  (set `self.Player` _asbp_slime_character))

(event `/Game/GPE/Possessible/BPI_Possessible.Attach`
  (bind (_returnvalue_location _returnvalue_rotation) (`KismetMathLibrary.BreakTransform` (`self.GetTransform`)))
  (bind _player (`self.Player`))
  (bind _player_2 (`self.Player`))
  (if (not (`self.Equiped`))
    (set `self.Equiped` true)
    (bind _returnvalue (`|SpawnActorFromClass` "/Game/Character/Slime/BP_Slime_Core.BP_Slime_Core_C" (`self.GetTransform` _player) "Undefined" "OverrideRootScale" null null))
    (set `/Game/Character/Slime/BP_Slime_Character.Core` _returnvalue _player)
    (set `/Game/Character/Slime/BP_Slime_Character.HeldObject` self _player)
    (`self.K2_SetActorTransform` _player_2 (`KismetMathLibrary.MakeTransform` _returnvalue_location _returnvalue_rotation) false false)
    (set `/Game/Character/Slime/BP_Slime_Character.InPossession` true _player_2)
    (`self.K2_AttachToComponent` (`/Game/Character/Slime/BP_Slime_Character.ItemAttach` _player_2) "None" "SnapToTarget" "SnapToTarget" "KeepWorld" false)))

(event `/Game/GPE/Possessible/BPI_Possessible.Detach`
  (bind _player (`self.Player`))
  (bind _core (`/Game/Character/Slime/BP_Slime_Character.Core` _player))
  (if (`self.Equiped`)
    (`self.K2_DetachFromActor` "KeepWorld" "KeepWorld" "KeepWorld")
    (`self.K2_SetActorLocation` (- (`self.K2_GetActorLocation`) (0.0 0.0 50.0)))
    (set `self.Equiped` false)
    (`self.K2_SetActorLocation` _player (`self.K2_GetActorLocation` _core) false false)
    (`self.K2_DestroyActor` _core)
    (set `/Game/Character/Slime/BP_Slime_Character.InPossession` false _player)
    (set `/Game/Character/Slime/BP_Slime_Character.HeldObject` null _player)
    (set `/Game/Character/Slime/BP_Slime_Character.Core` null _player)))

(fn `UserConstructionScript`)