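; BP_Possessible_drill is a possessible drill that switches a destruction field on and off.
; On BeginPlay it caches its child actor as a BP_destructionField.
; Action and StopAction set the Drilling flag and the field's Activated flag together, leaving any destruction logic to that field.
; DetectPlayer and UnsetPlayer are empty stubs, and construction adds nothing.
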(event `self.ReceiveBeginPlay`
  (bind _asbp_destruction_field (cast `/Game/GPE/Fields/BP_destructionField` (`ChildActorComponent.ChildActor` (`self.ChildActor`))))
  (set `self.DestroyFieldChild` _asbp_destruction_field))

(event `/Game/GPE/Possessible/BPI_Possessible.Action`
  (set `self.Drilling` true)
  (set `/Game/GPE/Fields/BP_destructionField.activated` true (`self.DestroyFieldChild`)))

(event `/Game/GPE/Possessible/BPI_Possessible.StopAction`
  (set `self.Drilling` false)
  (set `/Game/GPE/Fields/BP_destructionField.activated` false (`self.DestroyFieldChild`)))

(fn `DetectPlayer`
  (params (Slime :type "/Game/Character/BP_Slime_Character Object Reference"))
  (returns (Valid :type Boolean)))

(fn `UnsetPlayer`
  (params (Slime :type "/Game/Character/BP_Slime_Character Object Reference"))
  (returns (Valid :type Boolean)))

(fn `UserConstructionScript`)