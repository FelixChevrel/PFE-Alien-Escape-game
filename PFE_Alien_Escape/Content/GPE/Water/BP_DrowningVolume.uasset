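; BP_DrowningVolume is a water volume that flags when the player's slime character is inside it.
; On BeginPlay it caches player pawn 0 as a BP_Slime_Character.
; Its Box overlap events set that character's InWater flag on entry and clear it on exit, ignoring other actors.
; The volume contains no drowning logic itself, only the flag toggle.
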(event `self.ReceiveBeginPlay`
  (bind _asbp_slime_character (cast `/Game/Character/Slime/BP_Slime_Character` (`GameplayStatics.GetPlayerPawn` 0)))
  (set `self.PlayerRef` _asbp_slime_character))

(event `self.Box.OnComponentBeginOverlap`
  (params (OverlappedComponent :type "PrimitiveComponent Object Reference") (OtherActor :type "Actor Object Reference") (OtherComp :type "PrimitiveComponent Object Reference") (OtherBodyIndex :type Integer) (bFromSweep :type Boolean) (SweepResult :type "HitResult Structure (by ref)"))
  (bind _playerref (`self.PlayerRef`))
  (if (== OtherActor _playerref)
    (set `/Game/Character/Slime/BP_Slime_Character.InWater` true _playerref)))

(event `self.Box.OnComponentEndOverlap`
  (params (OverlappedComponent :type "PrimitiveComponent Object Reference") (OtherActor :type "Actor Object Reference") (OtherComp :type "PrimitiveComponent Object Reference") (OtherBodyIndex :type Integer))
  (bind _playerref (`self.PlayerRef`))
  (if (== _playerref OtherActor)
    (set `/Game/Character/Slime/BP_Slime_Character.InWater` false _playerref)))

(fn `UserConstructionScript`)